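; BP_VibratingPlatform is a demo-level platform actor whose plane shakes continuously, with strength scaled by a Vibrations value.
; Tick drives the plane's relative height, roll and pitch through the PerlinNoise helper, using time offsets to vary the axes, with fixed scale.
; The construction script starts a looping timer of about 60 Hz that calls EditorTick, which reuses the Tick logic, apparently to preview the motion in the editor.
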(event `self.ReceiveTick`
  (params (DeltaSeconds :type "Float (single-precision)"))
  (bind _vibrations (`self.Vibrations`))
  (`SceneComponent.K2_SetRelativeTransform` (`self.Plane`) (`KismetMathLibrary.MakeTransform` (`KismetMathLibrary.MakeVector` 0.0 0.0 (`self.Perlin Noise` 0.0 80.0 10.0 _vibrations)) (`KismetMathLibrary.MakeRotator` (`self.Perlin Noise` 1.0 80.0 3.0 _vibrations) (`self.Perlin Noise` 2.0 80.0 3.0 _vibrations)) (3.0 5.0 1.0)) false false :!label _label))

(event `/Game/CinematicCarRigLite/Blueprints/BI_CCRLiteEditorTick.EditorTick`
  (goto _label))

(fn `UserConstructionScript`
  (`KismetSystemLibrary.K2_SetTimer` null "EditorTick" 0.016667 true))